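; PC_UserController is a player controller that holds hotkeys for a screen fade effect and a temporary camera-change event.
; Keys 3 and 4 cast the HUD to BP_HUD and call PlayFadeEffect on its black widget with opposite boolean values.
; An event blends the view target to the controlled BP_VehicleF15 over several seconds, but the timer meant to trigger it is disconnected.
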(event Custom|temp_changecamera
  (bind _asbp_vehicle_f15 (Utilities|Casting|CastToBP_VehicleF15 (Pawn|GetControlledPawn)))
  (Game|Player|SetViewTargetwithBlend _asbp_vehicle_f15 5.0 "VTBlend_Linear" 0.0 false))

(event EventBeginPlay)

(event EventTick
  (params (DeltaSeconds :type Float%20%28single-precision%29)))

(event Input|KeyboardEvents|4
  (params (Key :type Key%20Structure :default "None"))
  (:Pressed
    (bind _asbp_hud (Utilities|Casting|CastToBP_HUD (HUD|GetHUD)))
    (Class|BlackWidget|PlayFadeEffect (Variables|/Script/Game5.PlayerHUD|GetGeneratedBlackWidget _asbp_hud) false)))

(event Input|KeyboardEvents|3
  (params (Key :type Key%20Structure :default "None"))
  (:Pressed
    (bind _asbp_hud (Utilities|Casting|CastToBP_HUD (HUD|GetHUD)))
    (Class|BlackWidget|PlayFadeEffect (Variables|/Script/Game5.PlayerHUD|GetGeneratedBlackWidget _asbp_hud) true)))

(fn ConstructionScript)