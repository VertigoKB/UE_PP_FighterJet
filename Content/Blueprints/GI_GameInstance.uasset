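; Game instance Blueprint that holds shared flight or movement state: thrust speed, current speed and the player's Z value.
; Each value has a plain getter and setter pair, with no validation, events or other logic.
; The file shows only this storage, not which Blueprints write or read the values.
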(fn GetGIThrustSpeed
  (return (Variables|Default|GetThrustSpeed)))

(fn SetGIThrustSpeed
  (params (ThrustParam :type Float%20%28double-precision%29))
  (Variables|Default|SetThrustSpeed ThrustParam))

(fn GetGICurrentSpeed
  (return (Variables|Default|GetCurrentSpeed)))

(fn SetGICurrentSpeed
  (params (CurrentSpeedParam :type Float%20%28double-precision%29))
  (Variables|Default|SetCurrentSpeed CurrentSpeedParam))

(fn GetGIPlayerZ
  (return (Variables|Default|GetPlayerZ)))

(fn SetGIPlayerZ
  (params (ZParam :type Float%20%28double-precision%29))
  (Variables|Default|SetPlayerZ ZParam))