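; BP_EnemyController is an AI controller for BP_Enemy that currently holds only setup and debug output.
; On BeginPlay it casts the controlled pawn to BP_Enemy and caches it as TempPawn.
; AI Perception target-updated and target-forgotten events print the actor's name, while Tick and perception-updated are empty.
; An unconnected debug print would show PosState position and sight flags, PlayerFinder target distance and current State.
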(event OnPerceptionUpdated(AIPerception)
  (params (UpdatedActors :type Array%20of%20Actor%20Object%20References)))

(event OnTargetPerceptionForgotten(AIPerception)
  (params (Actor :type Actor%20Object%20Reference))
  (Development|PrintString (Utilities|String|ToString(Text) (Utilities|Text|FormatText "Forgotten: {forgot} 
" (Utilities|GetDisplayName Actor)))))

(event OnTargetPerceptionUpdated(AIPerception)
  (params (Actor :type Actor%20Object%20Reference) (Stimulus :type AI%20Stimulus%20Structure))
  (Development|PrintString (Utilities|String|ToString(Text) (Utilities|Text|FormatText "Target: {target} 
" (Utilities|GetDisplayName Actor)))))

(event EventBeginPlay
  (bind _asbp_enemy (Utilities|Casting|CastToBP_Enemy (Pawn|GetControlledPawn)))
  (Variables|Default|SetTempPawn _asbp_enemy))

(event EventTick
  (params (DeltaSeconds :type Float%20%28single-precision%29)))

(fn ConstructionScript)